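; Player controller that routes input to the player's BP_Character and handles pausing.
; It caches the character on BeginPlay, then forwards jump, mouse pitch and yaw, and movement axes to it.
; Movement directions come from the forward and right vectors of the full control rotation.
; The pause input toggles game pause and adds or removes the paused HUD widget referenced on the character.
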(event EventBeginPlay
  ;[1 1 1] Setting To My Game Character
  (bind _asbp_character (Utilities|Casting|CastToBP_Character (Game|GetPlayerCharacter 0)))
  (Variables|Default|SetGameCharacter_Ref _asbp_character))

(event Input|ActionEvents|InputActionJump
  (params (Key :type Key%20Structure))
  ;[1 1 1] Player Rotation And Jump
  (:Pressed
    (Character|Jump (Variables|Default|GetGameCharacter_Ref))))

(event Input|ActionEvents|InputActionPause
  (params (Key :type Key%20Structure))
  (bind _gamecharacter_ref (Variables|Default|GetGameCharacter_Ref))
  (bind _pausedhud_ref (Variables|/Game/BluePrint/BP_Character.BP_Character_C|GetPausedHUD_Ref _gamecharacter_ref))
  ;[1 1 1] Pause System For Game
  (:Pressed
    (if (Game|IsGamePaused)
      (Game|SetGamePaused false)
      (Widget|RemovefromParent _pausedhud_ref)
      (else
        (Game|SetGamePaused true)
        (UserInterface|Viewport|AddtoViewport _pausedhud_ref 0)))))

(event Input|AxisEvents|InputAxisMouseRotationY
  (params (AxisValue :type Float%20%28single-precision%29))
  ;[1 1 1] Player Rotation And Jump
  (Pawn|Input|AddControllerPitchInput (Variables|Default|GetGameCharacter_Ref) AxisValue))

(event Input|AxisEvents|InputAxisMouseRotationX
  (params (AxisValue :type Float%20%28single-precision%29))
  ;[1 1 1] Player Rotation And Jump
  (Pawn|Input|AddControllerYawInput (Variables|Default|GetGameCharacter_Ref) AxisValue))

(event Input|AxisEvents|InputAxisMoveForwardAndBackWard
  (params (AxisValue :type Float%20%28single-precision%29))
  (bind _gamecharacter_ref (Variables|Default|GetGameCharacter_Ref))
  ;[1 1 1] Player Movement
  (Pawn|Input|AddMovementInput _gamecharacter_ref (Math|Vector|GetForwardVector (Pawn|GetControlRotation _gamecharacter_ref :!class /Script/Engine.Pawn)) AxisValue false))

(event Input|AxisEvents|InputAxisMoveRightAndLeft
  (params (AxisValue :type Float%20%28single-precision%29))
  (bind _gamecharacter_ref (Variables|Default|GetGameCharacter_Ref))
  ;[1 1 1] Player Movement
  (Pawn|Input|AddMovementInput _gamecharacter_ref (Math|Vector|GetRightVector (Pawn|GetControlRotation _gamecharacter_ref :!class /Script/Engine.Pawn)) AxisValue false))

(fn ConstructionScript)