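; Player character Blueprint that handles damage, death and creation of the pause HUD.
; AnyDamage subtracts from Health through a DoOnce gate that resets after a short delay, giving a brief invulnerability window between hits.
; When Health runs out, GameOver only prints a death message and the gate stays closed.
; BeginPlay creates the BP_Pause_HUD widget and stores its reference without displaying it.
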(event Custom|Game%20Over
  (Development|PrintString "Player Death"))

(event EventBeginPlay
  ;[1 1 1] Create Paused HUD
  (bind _returnvalue (UserInterface|CreateWidget "/Game/BluePrint/UI/BP_Pause_HUD.BP_Pause_HUD_C"))
  (Variables|Default|SetPausedHUD_Ref _returnvalue))

(event Game|Damage|EventAnyDamage
  (params (Damage :type Float%20%28single-precision%29) (DamageType :type Damage%20Type%20Object%20Reference) (InstigatedBy :type Controller%20Object%20Reference) (DamageCauser :type Actor%20Object%20Reference))
  ;[1 1 1] Getting Damage to Player
  (Utilities|FlowControl|DoOnce false :!label _label
    (:Completed
      (bind _output_get (Variables|Default|SetHealth (- (Variables|Default|GetHealth) Damage)))
      (if (<= _output_get 0.0)
        (CallFunction|GameOver)
        (else
          (Utilities|FlowControl|Delay 0.5)
          (goto _label Reset))))))

(fn ConstructionScript)