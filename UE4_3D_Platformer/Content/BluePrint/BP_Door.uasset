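; BP_Door is an exit door that opens only once the player has collected all three crystals and ends the game afterwards.
; Overlapping DoorTrigger sets a prompt message on BP_Character and enables input if the crystals are complete; leaving clears the message and disables input.
; The Open Door action plays a timeline that rotates the actor's yaw from its starting rotation, then calls GameOver on the character.
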(event OnComponentBeginOverlap(DoorTrigger)
  (params (OverlappedComponent :type Primitive%20Component%20Object%20Reference) (OtherActor :type Actor%20Object%20Reference) (OtherComp :type Primitive%20Component%20Object%20Reference) (OtherBodyIndex :type Integer) (bFromSweep :type Boolean) (SweepResult :type Hit%20Result%20Structure%20%28by%20ref%29))
  (bind _asbp_character (Utilities|Casting|CastToBP_Character OtherActor))
  (if (== (Variables|/Game/BluePrint/BP_Character.BP_Character_C|GetCrystalCollected _asbp_character) 3)
    (Variables|/Game/BluePrint/BP_Character.BP_Character_C|SetCrystalMassage _asbp_character "Press F to Open The Door")
    (Input|EnableInput (Game|GetPlayerController 0))
    (else
      (Variables|/Game/BluePrint/BP_Character.BP_Character_C|SetCrystalMassage _asbp_character "you need to collect all 3 crystals to open the door"))))

(event OnComponentEndOverlap(DoorTrigger)
  (params (OverlappedComponent :type Primitive%20Component%20Object%20Reference) (OtherActor :type Actor%20Object%20Reference) (OtherComp :type Primitive%20Component%20Object%20Reference) (OtherBodyIndex :type Integer))
  (bind _asbp_character (Utilities|Casting|CastToBP_Character OtherActor))
  (Variables|/Game/BluePrint/BP_Character.BP_Character_C|SetCrystalMassage _asbp_character "")
  (Input|DisableInput (Game|GetPlayerController 0)))

(event Input|ActionEvents|InputActionOpenDoor
  (params (Key :type Key%20Structure))
  (:Pressed
    (bind _output_get (Variables|Default|SetinitialRotate (Transformation|GetActorRotation)))
    (bind _rotatez (Timeline|Door%20TimeLine Play)
      (:Update
        (Transformation|SetActorRotation (Math|Rotator|MakeRotator (.Roll (Math|Rotator|BreakRotator _output_get)) (.Pitch (Math|Rotator|BreakRotator _output_get)) (- (.Yaw (Math|Rotator|BreakRotator _output_get)) _rotatez))))
      (:Finished
        (Default|GameOver (stale OnComponentBeginOverlap(DoorTrigger) _asbp_character))))))

(fn ConstructionScript)